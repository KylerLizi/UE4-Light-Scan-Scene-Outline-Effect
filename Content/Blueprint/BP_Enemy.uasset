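; BP_Enemy is an enemy Blueprint that runs a simple AI patrol between two positions.
; BeginPlay targets Position1 and starts the AIMove custom event, which calls AIMoveTo on itself.
; On success it waits briefly, uses a FlipFlop to alternate the target between Position2 and Position1, then calls AIMove again.
; The failure path is unhandled, so a failed move ends the patrol loop.
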(event `self.ReceiveBeginPlay`
  (set `self.TargetPos` (`self.Position1`))
  (`self.AIMove`))

(event `AIMove`
  ;[1 1 1] 简单AI巡逻
  (`|AIMoveTo` self (`self.TargetPos`) null
    (:`OnSuccess`
      (`KismetSystemLibrary.Delay` 1.0)
      (`/Engine/EditorBlueprintResources/StandardMacros.FlipFlop`
        (:`A`
          (set `self.TargetPos` (`self.Position2`)))
        (:`B`
          (set `self.TargetPos` (`self.Position1`))))
      (`self.AIMove`))))

(fn `UserConstructionScript`)